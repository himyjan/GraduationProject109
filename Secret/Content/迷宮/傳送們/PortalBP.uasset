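; Maze portal actor that teleports a ThirdPersonCharacter to its paired portal when hit, playing a 2D sound.
; On hit it searches all PortalBP actors for the same PortalIndex and opposite Enterence flag, so travel works both ways.
; The character is moved to that portal's ExitReference location.
; The construction script places the portal and exit point from variables and tints the portal through a dynamic material instance.
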(event Collision|EventHit
  (params (MyComp :type Primitive%20Component%20Object%20Reference) (Other :type Actor%20Object%20Reference) (OtherComp :type Primitive%20Component%20Object%20Reference) (bSelfMoved :type Boolean) (HitLocation :type Vector :default "0, 0, 0") (HitNormal :type Vector :default "0, 0, 0") (NormalImpulse :type Vector :default "0, 0, 0") (Hit :type Hit%20Result%20Structure%20%28by%20ref%29))
  (bind _asthird_person_character (Utilities|Casting|CastToThirdPersonCharacter Other))
  (Audio|PlaySound2D "/Game/音效/eating.eating" 1.0 1.0 0.0 0 0)
  (if (Variables|Default|GetEnterence)
    (bind _outactors (Actor|GetAllActorsOfClass "PortalBP_C"))
    (bind _array_element (Utilities|Array|ForEachLoopwithBreak _outactors :!label _label)
      (:LoopBody
        (if (and (== (Variables|PortalBP_C|GetPortal%20Index _array_element) (Variables|Default|GetPortal%20Index)) (not (Variables|PortalBP_C|GetEnterence _array_element)))
          (goto _label Break)))
      (:Completed
        (Transformation|SetActorLocation _asthird_person_character (Transformation|GetWorldLocation (Variables|PortalBP_C|GetExit%20reference _array_element)) false false)))
    (else
      (bind _outactors_2 (Actor|GetAllActorsOfClass "PortalBP_C"))
      (bind _array_element_2 (Utilities|Array|ForEachLoopwithBreak _outactors_2 :!label _label_2)
        (:LoopBody
          (if (and (== (Variables|PortalBP_C|GetPortal%20Index _array_element_2) (Variables|Default|GetPortal%20Index)) (and (not (Variables|Default|GetEnterence)) (Variables|PortalBP_C|GetEnterence _array_element_2)))
            (goto _label_2 Break)))
        (:Completed
          (Transformation|SetActorLocation _asthird_person_character (Transformation|GetWorldLocation (Variables|PortalBP_C|GetExit%20reference _array_element_2)) false false))))))

(fn ConstructionScript
  (bind _portal (Variables|Default|GetPortal))
  ;[1 1 1] 設置門和退出位置
  (Transformation|SetRelativeTransform (Variables|Default|GetPortal) (Variables|Default|GetPortal%20Transform) false false)
  (Transformation|SetRelativeLocation (Variables|Default|GetExit%20reference) (Variables|Default|GetExit%20Location) false false)
  ;[1 1 1] set portal color
  (bind _returnvalue (Rendering|Material|CreateDynamicMaterialInstance _portal 0 "/Game/迷宮/傳送們/PortalMat_Inst.PortalMat_Inst" "None" :!class /Script/Engine.PrimitiveComponent))
  (Rendering|Material|SetVectorParameterValue _returnvalue "color" (Variables|Default|Getcolor) :!class /Script/Engine.MaterialInstanceDynamic)
  (Rendering|Material|SetMaterial _portal 0 _returnvalue))